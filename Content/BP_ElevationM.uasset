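; Mortar-style elevation rig Blueprint that animates a tube and its supporting bipod through elevation and height changes.
; On BeginPlay, one timeline drives UpdateElevation, then a second drives UpdateBipodHeight; neither function is defined here.
; UpdateVisuals applies GeoParams by pitching the elevation and bipod pivots and Z-scaling the bipod mesh parent to its length.
; TriangleCheck is an uncalled debug helper that prints distances between the three pivot points.
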(event `self.ReceiveBeginPlay`
  (bind (_direction _elevation) (`Timeline|Timeline`)
    (:`Update`
      (`self.UpdateElevation` _elevation))
    (:`Finished`
      (bind (_direction_2 _height) (`Timeline|Timeline_0`)
        (:`Update`
          (`self.UpdateBipodHeight` _height))))))

(event `self.UpdateVisuals`
  (bind (_geoparams_elevationpivotheight _geoparams_bipodpivotoffset _geoparams_tubelength _geoparams_pivottobipodpivot _geoparams_bipodlength _geoparams_elevation _geoparams_bipodangle) (break `ElevationGeoParameters` (`self.GeoParams`)))
  (bind _elevationpivot (`self.ElevationPivot`))
  (bind (_relativerotation_roll _relativerotation_pitch _relativerotation_yaw) (`KismetMathLibrary.BreakRotator` (`SceneComponent.RelativeRotation` _elevationpivot)))
  (`|ExecutionSequence`
    (:`then_0`
      (`SceneComponent.K2_SetRelativeRotation` _elevationpivot (`KismetMathLibrary.MakeRotator` _relativerotation_roll (* (- _geoparams_elevation 90.0) -1.0) _relativerotation_yaw) false false)
      (`KismetSystemLibrary.PrintString` (`KismetStringLibrary.Conv_DoubleToString` _geoparams_bipodangle) false false (struct :`R` 1.0 :`B` 0.421799 :`A` 1.0) 0.0))
    (:`then_1`
      (`SceneComponent.K2_SetRelativeRotation` (`self.TubeBipodPivot`) (`KismetMathLibrary.MakeRotator` 0.0 _geoparams_bipodangle 180.0) false false))
    (:`then_2`
      (`SceneComponent.SetWorldScale3D` (`self.BipodMeshParent`) (`KismetMathLibrary.MakeVector` 1.0 1.0 (/ _geoparams_bipodlength 50.0))))))

(fn `TriangleCheck`
  (locals (PivotToBipodPivot :type "Float (double-precision)" :default 0.0) (PivotToBipodGround :type "Float (double-precision)" :default 0.0))
  (bind _returnvalue (`SceneComponent.K2_GetComponentLocation` (`self.BipodBottom`)))
  (bind _returnvalue_2 (`SceneComponent.K2_GetComponentLocation` (`self.TubeBipodPivot`)))
  (bind _returnvalue_3 (`SceneComponent.K2_GetComponentLocation` (`self.ElevationPivot`)))
  (bind _output_get (set `local.PivotToBipodPivot` (`KismetMathLibrary.VSize` (- _returnvalue_2 _returnvalue_3))))
  (bind _output_get_2 (set `local.PivotToBipodGround` (`KismetMathLibrary.VSize` (- _returnvalue _returnvalue_3))))
  (bind _output_get_3 (set `self.BipodHeight` (`KismetMathLibrary.VSize` (- _returnvalue_2 _returnvalue))))
  (`KismetSystemLibrary.PrintString` (`KismetStringLibrary.Concat_StrStr` "Pivot to bipod pivot: " (`KismetStringLibrary.Conv_DoubleToString` _output_get) " Pivot to bipod ground: " (`KismetStringLibrary.Conv_DoubleToString` _output_get_2) " Bipod Height: " (`KismetStringLibrary.Conv_DoubleToString` _output_get_3)) true true (struct :`G` 0.66 :`B` 1.0 :`A` 1.0) 10.0 "TriCheck"))

(fn `UserConstructionScript`)